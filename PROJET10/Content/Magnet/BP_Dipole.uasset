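; BP_Dipole is a two-pole magnet that attracts or repels nearby physics-simulating components.
; Each tick, ApplyInfluence runs for the south and north poles, scanning components that overlap that pole's range sphere and skipping its own poles.
; A differing slot-0 material means attraction, a matching one repulsion.
; Force falls off quadratically to zero at the sphere radius and is applied as equal, opposite halves at both centers of mass.
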(event `self.ReceiveTick`
  (params (DeltaSeconds :type "Float (single-precision)"))
  (bind _northactionrange (`self.NorthActionRange`))
  (`self.ApplyInfluence` (`self.SouthPole`) (`self.SouthActionRange`) (`SphereComponent.GetScaledSphereRadius` (`self.SouthActionRange`)))
  (`self.ApplyInfluence` (`self.NorthPole`) _northactionrange (`SphereComponent.GetScaledSphereRadius` _northactionrange)))

(fn `ApplyInfluence`
  (params (Pole :type "PrimitiveComponent Object Reference") (ActionRange :type "PrimitiveComponent Object Reference") (MaxDistance :type "Float (double-precision)"))
  (locals (L_Pole :type "PrimitiveComponent Object Reference") (L_ActionRange :type "PrimitiveComponent Object Reference") (L_ForeignPole :type "PrimitiveComponent Object Reference") (L_MaxDistance :type "Float (double-precision)"))
  (bind _l_maxdistance (`local.L_MaxDistance`))
  (bind _returnvalue (`PrimitiveComponent.GetCenterOfMass` (`local.L_ForeignPole`) "None"))
  (bind _returnvalue_2 (`PrimitiveComponent.GetCenterOfMass` (`local.L_Pole`) "None"))
  (bind _returnvalue_3 (- _returnvalue_2 _returnvalue))
  (bind _returnvalue_4 (/ (* (* (`KismetMathLibrary.Normal` _returnvalue_3) (* (`self.MaxForce`) (`KismetMathLibrary.Square` (/ (- _l_maxdistance (`KismetMathLibrary.FClamp` (`KismetMathLibrary.VSize` _returnvalue_3) 0.0 _l_maxdistance)) _l_maxdistance)))) (select `bool` (!= (`PrimitiveComponent.GetMaterial` (`local.L_ForeignPole`) 0) (`PrimitiveComponent.GetMaterial` (`local.L_Pole`) 0)) :`false` -1.0 :`true` 1.0 :!type "Float (single-precision)")) 2.0))
  (set `local.L_Pole` Pole)
  (set `local.L_ActionRange` ActionRange)
  (set `local.L_MaxDistance` MaxDistance)
  (for _array_element (`PrimitiveComponent.GetOverlappingComponents` (`local.L_ActionRange`))
    (bind _output_get (set `local.L_ForeignPole` _array_element))
    (if (and (!= _output_get (`self.SouthPole`)) (!= _output_get (`self.NorthPole`)))
      (if (`SceneComponent.IsSimulatingPhysics` (`local.L_ForeignPole`) "None")
        (`PrimitiveComponent.AddForceAtLocation` (`local.L_ForeignPole`) _returnvalue_4 _returnvalue "None"))
      (`PrimitiveComponent.AddForceAtLocation` (`local.L_Pole`) (* _returnvalue_4 -1.0) _returnvalue_2 "None"))))

(fn `UserConstructionScript`)